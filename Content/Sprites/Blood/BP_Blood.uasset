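; BP_Blood is a short-lived blood effect actor that turns to face the player before removing itself.
; On BeginPlay it waits a fraction of a second and then destroys itself.
; Each Tick it interpolates its rotation toward a look-at rotation at the player character, at a speed set by RotationSpeed, giving a billboard-style facing.
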(event EventBeginPlay
  (Utilities|FlowControl|Delay 0.3)
  (Actor|DestroyActor))

(event Collision|EventActorBeginOverlap
  (params (OtherActor :type Actor%20Object%20Reference)))

(event EventTick
  (params (DeltaSeconds :type Float%20%28single-precision%29))
  (Transformation|SetActorRotation (Math|Interpolation|RInterpTo (Transformation|GetActorRotation) (Math|Rotator|FindLookatRotation (Transformation|GetActorLocation) (Transformation|GetActorLocation (Game|GetPlayerCharacter 0))) (Utilities|Time|GetWorldDeltaSeconds) (Variables|Default|GetRotationSpeed))))

(fn ConstructionScript)