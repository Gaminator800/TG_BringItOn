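; Base enemy for a first-person shooter, drawn as a directional Paper2D sprite, with melee, ranged and optional boss behavior.
; Tick derives state from velocity and attacks, then picks flipbook and rotation from the player's angle and side via dot products.
; Sight, noise and damage set the CanSeePlayer blackboard key; attacks use line traces or spawned projectiles.
; Death stops AI, plays corpse flipbooks, credits a kill or signals boss defeat, then destroys the actor.
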(event OnSeePawn(PawnSensing)
  (params (Pawn :type Pawn%20Object%20Reference))
  ;[0.15 0.15 0.15 0.5] HandleEnemyVision
  (Utilities|Casting|CastToBP_FirstPersonCharacter Pawn)
  (Variables|DoNotEdit|SetCanSeePlayer true)
  (AI|Components|Blackboard|SetValueasBool (AI|GetBlackboard 0) (Utilities|Name|MakeLiteralName "CanSeePlayer") true)
  (Utilities|FlowControl|RetriggerableDelay 0.7)
  (Variables|DoNotEdit|SetCanSeePlayer false)
  (AI|Components|Blackboard|SetValueasBool (AI|GetBlackboard 0) (Utilities|Name|MakeLiteralName "CanSeePlayer") false))

(event OnHearNoise(PawnSensing)
  (params (Instigator :type Pawn%20Object%20Reference) (Location :type Vector%20%28by%20ref%29 :default "0, 0, 0") (Volume :type Float%20%28single-precision%29))
  ;[0.15 0.15 0.15 0.5] HandleEnemyDamage
  (if (== Instigator (Game|GetPlayerCharacter 0))
    (Variables|DoNotEdit|SetCanSeePlayer true)
    (AI|Components|Blackboard|SetValueasBool (AI|GetBlackboard 0) (Utilities|Name|MakeLiteralName "CanSeePlayer") true)
    (if (Variables|DoNotEdit|GetPain?)
      (Variables|DoNotEdit|SetPain? true)
      (CallFunction|PlayPain)
      (Utilities|FlowControl|Delay 0.6)
      (CallFunction|ResetPainSound)
      (else
        (Variables|DoNotEdit|SetPain? false)))))

(event Custom|SpawnProjectile
  ;[0.15 0.15 0.15 0.5] Attack Systems
  ;;[0.15 0 0 0.5] RangedAttack
  (Variables|DoNotEdit|SetIsAttacking? true)
  (Variables|DoNotEdit|SetAttackState "NewEnumerator1")
  (Audio|PlaySoundatLocation (Variables|Edit|GetFiringSound) (Transformation|GetActorLocation) "0, 0, 0" 1.0 (Variables|Edit|GetPitch%20Multiplier) 0.0 0 0 0 0)
  (Components|Movement|StopMovementImmediately (Variables|Character|GetCharacterMovement))
  (Game|SpawnActorfromClass "/Game/Blueprints/Projectiles/BP_Enemy_Projectile.BP_Enemy_Projectile_C" (Transformation|GetWorldTransform (Variables|Default|GetProjectileSpawn)) "Undefined" "MultiplyWithRoot" 0 (Variables|Edit|GetProjectile%20Speed) (Variables|Edit|GetProjectile%20Damage) 0)
  (Utilities|FlowControl|RetriggerableDelay (+ (Variables|Edit|GetFireRate) 0.1))
  (Variables|DoNotEdit|SetIsAttacking? false))

(event Custom|MeleeAttack
  (bind _returnvalue (Transformation|GetActorLocation))
  (bind _returnvalue_2 (Game|GetPlayerCharacter 0))
  ;[0.15 0.15 0.15 0.5] Attack Systems
  ;;[0.15 0 0 0.5] MeleeAttack
  (Variables|DoNotEdit|SetIsAttacking? true)
  (Variables|DoNotEdit|SetAttackState "NewEnumerator0")
  (bind _outhit (Collision|LineTraceForObjects _returnvalue (+ _returnvalue (* (Transformation|GetActorForwardVector) 1.5e+02)) (Utilities|Array|MakeArray "ObjectTypeQuery3") false (Utilities|Array|MakeArray self) "None"))
  (if (== (.HitActor (Collision|BreakHitResult _outhit)) _returnvalue_2)
    (Audio|PlaySoundatLocation (Variables|Edit|GetMeleeSound) (Transformation|GetActorLocation) "0, 0, 0" 1.0 (Variables|Edit|GetMeleeSoundPitch) (Variables|Edit|GetMeleeSoundStartTime) 0 0 0 0)
    (Game|Damage|ApplyDamage _returnvalue_2 (Variables|Edit|GetEnemyDamage) 0 0))
  (Utilities|FlowControl|RetriggerableDelay (+ (Variables|Edit|GetMeleeRate) 0.1))
  (Variables|DoNotEdit|SetIsAttacking? false))

(event Custom|HandleDeath
  (bind _returnvalue (Transformation|GetActorTransform))
  (bind _paperflipbook (Variables|Default|GetPaperFlipbook))
  ;[0.15 0.15 0.15 0.5] HandleEnemyDeathSystem
  (Transformation|SetActorRotation (Math|Rotator|MakeRotator 0.0 0.0 (.yaw (Math|Rotator|FindLookatRotation (Transformation|GetActorLocation) (Transformation|GetActorLocation (Game|GetPlayerCharacter 0))))))
  (Utilities|FlowControl|DoOnce false
    (:Completed
      (AI|Logic|StopLogic (Variables|/Script/AIModule.AIController|GetBrainComponent (AI|GetAIController self)) "IsDead?")
      (Pawn|Components|CharacterMovement|SetMovementMode (Variables|Character|GetCharacterMovement) "MOVE_Falling" 0)
      (Collision|SetCollisionEnabled (Variables|Collision|GetCapsuleComponent) "NoCollision")
      (Components|Activation|Deactivate (Variables|Character|GetCharacterMovement))
      (Transformation|SetRelativeRotation _paperflipbook "0.000000,-90.000000,0.000000" false false)
      (Sprite|SetFlipbook _paperflipbook (Variables|FlipBooks|GetEnemyDeathFlipBook))
      (Audio|PlaySound2D (Variables|Edit|GetDeathSound) 1.0 (Variables|Edit|GetDeathPitchMultiplier) 0.0 0 0)
      (Utilities|FlowControl|Delay (- (Class|PaperFlipbookComponent|GetFlipbookLength (Variables|Default|GetPaperFlipbook)) 0.2))
      (Transformation|AddActorLocalOffset (Variables|Edit|GetDeadPosition) false false)
      (Sprite|SetFlipbook (Variables|Default|GetPaperFlipbook) (Variables|FlipBooks|GetEnemyBodyFlipBook))
      (if (Variables|Edit|GetIsBoss?)
        (Default|CallBossDefeated)
        (Utilities|FlowControl|Delay 4.0 :!label _label)
        (Actor|DestroyActor)
        (if (Variables|Edit|GetIsBoss?)
          (Audio|PlaySound2D "/Game/SFX/Weapons/Pistol/BFG_Fire.BFG_Fire" 1.0 -0.5 0.5 0 0)
          (Game|SpawnActorfromClass "/Game/Blueprints/Projectiles/BP_TeleportFX.BP_TeleportFX_C" (Math|Transform|MakeTransform (Math|Vector|MakeVector (.x (.location _returnvalue)) (.y (.location _returnvalue)) (+ (.z (.location _returnvalue)) 5e+01)) (.rotation _returnvalue) "1.000000,1.000000,1.000000") "Undefined" "MultiplyWithRoot" 0 0))
        (else
          (Utilities|FlowControl|Sequence
            (:then_0
              (bind _asbp_first_person_character (Utilities|Casting|CastToBP_FirstPersonCharacter (Game|GetPlayerCharacter 0)))
              (Math|Integer|IncrementInt (Variables|/Game/FirstPerson/Blueprints/BP_FirstPersonCharacter.BP_FirstPersonCharacter_C|GetKills _asbp_first_person_character)))
            (:then_1
              (goto _label))))))))

(event Custom|ResetPainSound
  (Utilities|FlowControl|DoOnce false) ; enters at Reset
)

(event Custom|PlayPain
  (Utilities|FlowControl|DoOnce false
    (:Completed
      (Audio|PlaySound2D (Variables|Edit|GetPainSound) 1.0 1.0 0.0 0 0))))

(event Game|Damage|EventAnyDamage
  (params (Damage :type Float%20%28single-precision%29) (DamageType :type Damage%20Type%20Object%20Reference) (InstigatedBy :type Controller%20Object%20Reference) (DamageCauser :type Actor%20Object%20Reference))
  ;[0.15 0.15 0.15 0.5] HandleEnemyDamage
  (bind _output_get (Variables|Edit|SetHealth (- (Variables|Edit|GetHealth) Damage)))
  (Variables|DoNotEdit|SetPain? true)
  (if (<= _output_get 0.0)
    (Variables|DoNotEdit|SetIsDead? true)
    (Variables|DoNotEdit|SetPain? false)
    (else
      (Variables|DoNotEdit|SetCanSeePlayer true)
      (AI|Components|Blackboard|SetValueasBool (AI|GetBlackboard 0) (Utilities|Name|MakeLiteralName "CanSeePlayer") true)
      (if (Variables|DoNotEdit|GetPain?)
        (Variables|DoNotEdit|SetPain? true)
        (CallFunction|PlayPain)
        (Utilities|FlowControl|Delay 0.6)
        (CallFunction|ResetPainSound)
        (else
          (Variables|DoNotEdit|SetPain? false))))))

(event EventTick
  (params (DeltaSeconds :type Float%20%28single-precision%29))
  (bind _returnvalue (|HandleEnemyState*CalculateEnemyDegrees))
  (|SetEnemyRotation&FlipBook _returnvalue))

(fn ConstructionScript)