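; BP_Dialogue is a placeable trigger volume that shows a one-time speech line when the first-person character walks into it.
; The construction script sizes the Box from an extent variable.
; On the first overlap it creates a WBP_DialogueScreen with its Speech value, plays the widget's appear and timed disappear, then removes it and destroys itself.
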(event OnComponentBeginOverlap(Box)
  (params (OverlappedComponent :type Primitive%20Component%20Object%20Reference) (OtherActor :type Actor%20Object%20Reference) (OtherComp :type Primitive%20Component%20Object%20Reference) (OtherBodyIndex :type Integer) (bFromSweep :type Boolean) (SweepResult :type Hit%20Result%20Structure%20%28by%20ref%29))
  (Utilities|Casting|CastToBP_FirstPersonCharacter OtherActor)
  (Utilities|FlowControl|DoOnce false
    (:Completed
      (bind _returnvalue (UserInterface|CreateWidget "/Game/Blueprints/UI/WBP_DialogueScreen.WBP_DialogueScreen_C" 0 (Variables|Default|GetSpeech)))
      (UserInterface|Viewport|AddtoViewport _returnvalue 0)
      (Default|Appear _returnvalue)
      (Utilities|FlowControl|Delay 5.0)
      (Default|Disappear _returnvalue)
      (Utilities|FlowControl|Delay 0.5)
      (Widget|RemovefromParent _returnvalue)
      (Actor|DestroyActor))))

(event EventBeginPlay)

(event Collision|EventActorBeginOverlap
  (params (OtherActor :type Actor%20Object%20Reference)))

(event EventTick
  (params (DeltaSeconds :type Float%20%28single-precision%29)))

(fn ConstructionScript
  (Components|Box|SetBoxExtent (Variables|Default|GetBox) (Variables|Default|GetIn%20Box%20Extent) true))