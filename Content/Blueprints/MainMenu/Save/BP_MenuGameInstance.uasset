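; Game instance that holds and persists the player's menu settings for controls, audio, display and graphics quality across sessions.
; On Init it loads the Save1 slot into a BP_TGBION_SaveGame and copies its values into its own variables, or creates and saves a new save object if none exists.
; SaveGame copies the current variables back into that object and writes the slot, but only when the save already exists.
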(event Custom|SaveGame
  (bind _saveref (Variables|Default|GetSaveRef))
  (bind _returnvalue (SaveGame|DoesSaveGameExist "Save1"))
  (if _returnvalue
    (Utilities|FlowControl|Sequence
      (:then_0
        (Variables|/Game/Blueprints/MainMenu/Save/BP_TGBION_SaveGame.BP_TGBION_SaveGame_C|SetLookSensitivityY _saveref (Variables|Default|GetLookSensitivityY))
        (Variables|/Game/Blueprints/MainMenu/Save/BP_TGBION_SaveGame.BP_TGBION_SaveGame_C|SetLookSensitivityX _saveref (Variables|Default|GetLookSensitivityX))
        (Variables|/Game/Blueprints/MainMenu/Save/BP_TGBION_SaveGame.BP_TGBION_SaveGame_C|SetAimingInvertY _saveref (Variables|Default|GetAimingInvertY))
        (Variables|/Game/Blueprints/MainMenu/Save/BP_TGBION_SaveGame.BP_TGBION_SaveGame_C|SetAimingInvertX _saveref (Variables|Default|GetAimingInvertX))
        (Variables|/Game/Blueprints/MainMenu/Save/BP_TGBION_SaveGame.BP_TGBION_SaveGame_C|SetMasterVolume _saveref (Variables|Default|GetMasterVolume))
        (Variables|/Game/Blueprints/MainMenu/Save/BP_TGBION_SaveGame.BP_TGBION_SaveGame_C|SetSFXVolume _saveref (Variables|Default|GetSFXVolume))
        (Variables|/Game/Blueprints/MainMenu/Save/BP_TGBION_SaveGame.BP_TGBION_SaveGame_C|SetMusicVolume _saveref (Variables|Default|GetMusicVolume))
        (Variables|/Game/Blueprints/MainMenu/Save/BP_TGBION_SaveGame.BP_TGBION_SaveGame_C|SetResolution _saveref (Variables|Default|GetResolution)))
      (:then_1
        (Variables|/Game/Blueprints/MainMenu/Save/BP_TGBION_SaveGame.BP_TGBION_SaveGame_C|SetWindowMode _saveref (Variables|Default|GetWindowMode))
        (Variables|/Game/Blueprints/MainMenu/Save/BP_TGBION_SaveGame.BP_TGBION_SaveGame_C|SetVSync _saveref (Variables|Default|GetVSync))
        (Variables|/Game/Blueprints/MainMenu/Save/BP_TGBION_SaveGame.BP_TGBION_SaveGame_C|SetBrightness _saveref (Variables|Default|GetBrightness))
        (Variables|/Game/Blueprints/MainMenu/Save/BP_TGBION_SaveGame.BP_TGBION_SaveGame_C|SetMotionBlur _saveref (Variables|Default|GetMotionBlur))
        (Variables|/Game/Blueprints/MainMenu/Save/BP_TGBION_SaveGame.BP_TGBION_SaveGame_C|SetVignette _saveref (Variables|Default|GetVignette))
        (Variables|/Game/Blueprints/MainMenu/Save/BP_TGBION_SaveGame.BP_TGBION_SaveGame_C|SetViewDistance _saveref (Variables|Default|GetViewDistance))
        (Variables|/Game/Blueprints/MainMenu/Save/BP_TGBION_SaveGame.BP_TGBION_SaveGame_C|SetAntiAliasing _saveref (Variables|Default|GetAntiAliasing))
        (Variables|/Game/Blueprints/MainMenu/Save/BP_TGBION_SaveGame.BP_TGBION_SaveGame_C|SetShadows _saveref (Variables|Default|GetShadows))
        (Variables|/Game/Blueprints/MainMenu/Save/BP_TGBION_SaveGame.BP_TGBION_SaveGame_C|SetTextures _saveref (Variables|Default|GetTextures)))
      (:then_2
        (SaveGame|SaveGametoSlot (Variables|Default|GetSaveRef) "Save1")))))

(event EventInit
  (bind _returnvalue (SaveGame|DoesSaveGameExist "Save1"))
  (if _returnvalue
    (bind _returnvalue_2 (SaveGame|LoadGamefromSlot "Save1"))
    (bind _asbp_tgbion_save_game (Utilities|Casting|CastToBP_TGBION_SaveGame _returnvalue_2))
    (bind _output_get (Variables|Default|SetSaveRef _asbp_tgbion_save_game))
    (Utilities|FlowControl|Sequence
      (:then_0
        (Variables|Default|SetLookSensitivityY (Variables|/Game/Blueprints/MainMenu/Save/BP_TGBION_SaveGame.BP_TGBION_SaveGame_C|GetLookSensitivityY _output_get))
        (Variables|Default|SetLookSensitivityX (Variables|/Game/Blueprints/MainMenu/Save/BP_TGBION_SaveGame.BP_TGBION_SaveGame_C|GetLookSensitivityX _output_get))
        (Variables|Default|SetAimingInvertY (Variables|/Game/Blueprints/MainMenu/Save/BP_TGBION_SaveGame.BP_TGBION_SaveGame_C|GetAimingInvertY _output_get))
        (Variables|Default|SetAimingInvertX (Variables|/Game/Blueprints/MainMenu/Save/BP_TGBION_SaveGame.BP_TGBION_SaveGame_C|GetAimingInvertX _output_get))
        (Variables|Default|SetMasterVolume (Variables|/Game/Blueprints/MainMenu/Save/BP_TGBION_SaveGame.BP_TGBION_SaveGame_C|GetMasterVolume _output_get))
        (Variables|Default|SetSFXVolume (Variables|/Game/Blueprints/MainMenu/Save/BP_TGBION_SaveGame.BP_TGBION_SaveGame_C|GetSFXVolume _output_get))
        (Variables|Default|SetMusicVolume (Variables|/Game/Blueprints/MainMenu/Save/BP_TGBION_SaveGame.BP_TGBION_SaveGame_C|GetMusicVolume _output_get))
        (Variables|Default|SetResolution (Variables|/Game/Blueprints/MainMenu/Save/BP_TGBION_SaveGame.BP_TGBION_SaveGame_C|GetResolution _output_get)))
      (:then_1
        (Variables|Default|SetWindowMode (Variables|/Game/Blueprints/MainMenu/Save/BP_TGBION_SaveGame.BP_TGBION_SaveGame_C|GetWindowMode _output_get))
        (Variables|Default|SetVSync (Variables|/Game/Blueprints/MainMenu/Save/BP_TGBION_SaveGame.BP_TGBION_SaveGame_C|GetVSync _output_get))
        (Variables|Default|SetBrightness (Variables|/Game/Blueprints/MainMenu/Save/BP_TGBION_SaveGame.BP_TGBION_SaveGame_C|GetBrightness _output_get))
        (Variables|Default|SetMotionBlur (Variables|/Game/Blueprints/MainMenu/Save/BP_TGBION_SaveGame.BP_TGBION_SaveGame_C|GetMotionBlur _output_get))
        (Variables|Default|SetVignette (Variables|/Game/Blueprints/MainMenu/Save/BP_TGBION_SaveGame.BP_TGBION_SaveGame_C|GetVignette _output_get))
        (Variables|Default|SetViewDistance (Variables|/Game/Blueprints/MainMenu/Save/BP_TGBION_SaveGame.BP_TGBION_SaveGame_C|GetViewDistance _output_get))
        (Variables|Default|SetAntiAliasing (Variables|/Game/Blueprints/MainMenu/Save/BP_TGBION_SaveGame.BP_TGBION_SaveGame_C|GetAntiAliasing _output_get))
        (Variables|Default|SetShadows (Variables|/Game/Blueprints/MainMenu/Save/BP_TGBION_SaveGame.BP_TGBION_SaveGame_C|GetShadows _output_get))
        (Variables|Default|SetTextures (Variables|/Game/Blueprints/MainMenu/Save/BP_TGBION_SaveGame.BP_TGBION_SaveGame_C|GetTextures _output_get))))
    (else
      (bind _returnvalue_3 (SaveGame|CreateSaveGameObject "/Game/Blueprints/MainMenu/Save/BP_TGBION_SaveGame.BP_TGBION_SaveGame_C"))
      (bind _output_get_2 (Variables|Default|SetSaveRef _returnvalue_3))
      (SaveGame|SaveGametoSlot _output_get_2 "Save1"))))