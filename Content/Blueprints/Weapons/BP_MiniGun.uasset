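; BP_MiniGun is an automatic weapon that fires repeatedly on a looping timer while shooting is active.
; ShootWeapon starts the timer through a resettable DoOnce, so repeat calls cannot stack timers.
; Each tick of the timer checks and spends ammo, fires, plays sound and sets the firing flipbook.
; StopShooting or running out of ammo clears the timer, restores the idle flipbook and resets the DoOnce.
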(event Custom|FireMiniGun
  (bind _hasammo (CallFunction|HasEnoughAmmo?))
  (if _hasammo
    (CallFunction|DecreaseAmmo)
    (CallFunction|FireWeapon)
    (CallFunction|PlayWeaponSound)
    (Sprite|SetFlipbook (Variables|Default|GetWeaponFlipBook) "/Game/Sprites/Weapons/MiniGun/MiniGun_Fire.MiniGun_Fire")
    (else
      (Utilities|Time|ClearandInvalidateTimerbyHandle (Variables|Default|GetMiniGunEvent))
      (Sprite|SetFlipbook (Variables|Default|GetWeaponFlipBook) "/Game/Sprites/Weapons/MiniGun/MiniGun_Idle.MiniGun_Idle")
      (CallFunction|ResetFire))))

(event Custom|ResetFire
  (Utilities|FlowControl|DoOnce false) ; enters at Reset
)

(event EventBeginPlay
  (|CallParentFunction) ; This node is disabled and will not be called.\nDrag off pins to build functionality.
)

(event Collision|EventActorBeginOverlap
  (params (OtherActor :type Actor%20Object%20Reference))
  (|CallParentFunction OtherActor) ; This node is disabled and will not be called.\nDrag off pins to build functionality.
)

(event EventTick
  (params (DeltaSeconds :type Float%20%28single-precision%29))
  (|CallParentFunction DeltaSeconds) ; This node is disabled and will not be called.\nDrag off pins to build functionality.
)

(event EventShootWeapon
  (Utilities|FlowControl|DoOnce false
    (:Completed
      (bind _returnvalue (Utilities|Time|SetTimerbyEvent (delegate Custom|FireMiniGun) 0.15 true))
      (Variables|Default|SetMiniGunEvent _returnvalue))))

(event EventStopShooting
  (Utilities|Time|ClearandInvalidateTimerbyHandle (Variables|Default|GetMiniGunEvent))
  (Sprite|SetFlipbook (Variables|Default|GetWeaponFlipBook) "/Game/Sprites/Weapons/MiniGun/MiniGun_Idle.MiniGun_Idle")
  (CallFunction|ResetFire))

(fn ConstructionScript
  (|CallParentFunction))