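; BP_Shotgun is a shotgun weapon that uses Paper2D flipbooks for its firing and idle visuals.
; ShootWeapon checks ammo, then passes a DoOnce gate to decrease ammo, fire, play the sound and switch to the fire flipbook.
; After a delay equal to that flipbook's length, it restores the idle flipbook and calls ResetWeaponFire to reopen the gate, so the animation sets the fire rate.
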(event Custom|ResetWeaponFire
  (bind _weaponflipbook (Variables|Default|GetWeaponFlipBook))
  (Utilities|FlowControl|DoOnce false) ; enters at Reset
)

(event EventBeginPlay
  (|CallParentFunction) ; This node is disabled and will not be called.\nDrag off pins to build functionality.
)

(event Collision|EventActorBeginOverlap
  (params (OtherActor :type Actor%20Object%20Reference))
  (|CallParentFunction OtherActor) ; This node is disabled and will not be called.\nDrag off pins to build functionality.
)

(event EventTick
  (params (DeltaSeconds :type Float%20%28single-precision%29))
  (|CallParentFunction DeltaSeconds) ; This node is disabled and will not be called.\nDrag off pins to build functionality.
)

(event EventShootWeapon
  (bind _weaponflipbook (Variables|Default|GetWeaponFlipBook))
  (bind _hasammo (CallFunction|HasEnoughAmmo?))
  (if _hasammo
    (Utilities|FlowControl|DoOnce false
      (:Completed
        (CallFunction|DecreaseAmmo)
        (CallFunction|FireWeapon)
        (CallFunction|PlayWeaponSound)
        (Sprite|SetFlipbook _weaponflipbook "/Game/Sprites/Weapons/Shotgun/Shotgun_Fire.Shotgun_Fire")
        (Utilities|FlowControl|Delay (Class|PaperFlipbookComponent|GetFlipbookLength _weaponflipbook))
        (Sprite|SetFlipbook (Variables|Default|GetWeaponFlipBook) "/Game/Sprites/Weapons/Shotgun/Shotgun_Idle.Shotgun_Idle")
        (CallFunction|ResetWeaponFire)))))

(fn ConstructionScript
  (|CallParentFunction))