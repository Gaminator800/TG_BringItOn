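; BP_BFG is the BFG weapon Blueprint, a flipbook-animated gun that fires a projectile at a cost of 30 Cell ammo.
; ShootWeapon checks the player's ammo, plays the sound and fire flipbook, then launches the projectile after the animation's length.
; It then returns to the idle flipbook, deducts ammo and updates the HUD.
; A DoOnce gate, reset when the sequence finishes, blocks overlapping shots.
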(event Custom|ResetDoOnce
  (bind _playercharacterref (Variables|Default|GetPlayerCharacterRef))
  (bind _weaponflipbook (Variables|Default|GetWeaponFlipBook))
  (Utilities|FlowControl|DoOnce false) ; enters at Reset
)

(event EventBeginPlay
  (|CallParentFunction) ; This node is disabled and will not be called.\nDrag off pins to build functionality.
)

(event Collision|EventActorBeginOverlap
  (params (OtherActor :type Actor%20Object%20Reference))
  (|CallParentFunction OtherActor) ; This node is disabled and will not be called.\nDrag off pins to build functionality.
)

(event EventTick
  (params (DeltaSeconds :type Float%20%28single-precision%29))
  (|CallParentFunction DeltaSeconds) ; This node is disabled and will not be called.\nDrag off pins to build functionality.
)

(event EventShootWeapon
  (bind _playercharacterref (Variables|Default|GetPlayerCharacterRef))
  (bind _weaponflipbook (Variables|Default|GetWeaponFlipBook))
  (if (>= (Variables|/Game/FirstPerson/Blueprints/BP_FirstPersonCharacter.BP_FirstPersonCharacter_C|GetCell (Variables|Default|GetPlayerCharacterRef)) 30)
    (Utilities|FlowControl|DoOnce false
      (:Completed
        (CallFunction|PlayWeaponSound)
        (Sprite|SetFlipbook _weaponflipbook "/Game/Sprites/Weapons/BFG/BFG_Fire.BFG_Fire")
        (Utilities|FlowControl|Delay (Class|PaperFlipbookComponent|GetFlipbookLength _weaponflipbook))
        (CallFunction|FireProjectile)
        (Sprite|SetFlipbook (Variables|Default|GetWeaponFlipBook) "/Game/Sprites/Weapons/BFG/BFG_Idle.BFG_Idle")
        (Variables|/Game/FirstPerson/Blueprints/BP_FirstPersonCharacter.BP_FirstPersonCharacter_C|SetCell _playercharacterref (- (Variables|/Game/FirstPerson/Blueprints/BP_FirstPersonCharacter.BP_FirstPersonCharacter_C|GetCell _playercharacterref) 30))
        (Default|UpdateCellAmmo (Variables|/Game/FirstPerson/Blueprints/BP_FirstPersonCharacter.BP_FirstPersonCharacter_C|GetPlayerHUD _playercharacterref))
        (CallFunction|ResetDoOnce)))))

(fn ConstructionScript
  (|CallParentFunction))