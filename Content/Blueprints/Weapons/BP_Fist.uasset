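; BP_Fist is a melee fist weapon Blueprint that performs a punch attack.
; ShootWeapon fires the weapon, plays its sound and switches the flipbook to the punch animation.
; After a delay equal to the flipbook's length it returns to the idle flipbook and calls ResetAttack.
; A DoOnce gate blocks repeat punches until that reset.
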(event Custom|ResetAttack
  (bind _weaponflipbook (Variables|Default|GetWeaponFlipBook))
  (Utilities|FlowControl|DoOnce false) ; enters at Reset
)

(event EventBeginPlay
  (|CallParentFunction) ; This node is disabled and will not be called.\nDrag off pins to build functionality.
)

(event Collision|EventActorBeginOverlap
  (params (OtherActor :type Actor%20Object%20Reference))
  (|CallParentFunction OtherActor) ; This node is disabled and will not be called.\nDrag off pins to build functionality.
)

(event EventTick
  (params (DeltaSeconds :type Float%20%28single-precision%29))
  (|CallParentFunction DeltaSeconds) ; This node is disabled and will not be called.\nDrag off pins to build functionality.
)

(event EventShootWeapon
  (bind _weaponflipbook (Variables|Default|GetWeaponFlipBook))
  (Utilities|FlowControl|DoOnce false
    (:Completed
      (CallFunction|FireWeapon)
      (CallFunction|PlayWeaponSound)
      (Sprite|SetFlipbook _weaponflipbook "/Game/Sprites/Weapons/Punch/Fixed/Gaminator_Punch_Fixed.Gaminator_Punch_Fixed")
      (Utilities|FlowControl|Delay (Class|PaperFlipbookComponent|GetFlipbookLength _weaponflipbook))
      (Sprite|SetFlipbook (Variables|Default|GetWeaponFlipBook) "/Game/Sprites/Weapons/Punch/Fixed/Gaminator_Punch_Idle_Fixed.Gaminator_Punch_Idle_Fixed")
      (CallFunction|ResetAttack))))

(fn ConstructionScript
  (|CallParentFunction))