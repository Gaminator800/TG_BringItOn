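; BP_TriggerDoor is a one-shot door that rises and then removes itself when its OpenDoor event is called.
; A DoOnce gate plays the opening sound and starts the DoorTL timeline, which raises the Cube along Z using the ToTheTop offset.
; Each update lerps from the Cube's current height rather than a stored start position, so the movement accumulates.
; The actor destroys itself shortly after the timeline finishes.
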(event Custom|OpenDoor
  (bind _cube (Variables|Default|GetCube))
  (bind _returnvalue (Transformation|GetWorldLocation _cube))
  (Utilities|FlowControl|DoOnce false
    (:Completed
      (Audio|PlaySoundatLocation "/Game/SFX/Door_Open_SFX.Door_Open_SFX" (Transformation|GetActorLocation) "0, 0, 0" 1.0 1.0 0.0 0 0 0 0)
      (bind _alpha (Timeline|DoorTL PlayFromStart)
        (:Update
          (Transformation|SetWorldLocation _cube (Math|Vector|MakeVector (.x _returnvalue) (.y _returnvalue) (Math|Float|Lerp (.z _returnvalue) (+ (.z _returnvalue) (Variables|Default|GetToTheTop)) _alpha)) false false))
        (:Finished
          (Utilities|FlowControl|Delay 0.2)
          (Actor|DestroyActor))))))

(event EventBeginPlay)

(event Collision|EventActorBeginOverlap
  (params (OtherActor :type Actor%20Object%20Reference)))

(event EventTick
  (params (DeltaSeconds :type Float%20%28single-precision%29)))

(fn ConstructionScript)