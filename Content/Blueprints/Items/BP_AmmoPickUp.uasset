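; Ammo pickup actor that grants bullets, shells, rockets or cells to the first-person player character.
; The construction script picks the Paper2D sprite from AmmoType and scales it, and Tick yaws the actor to face the player like a billboard.
; On the first box overlap by the player, it adds clamped ammo, updates the matching HUD counter, plays a pickup sound and destroys itself.
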(event OnComponentBeginOverlap(Box)
  (params (OverlappedComponent :type Primitive%20Component%20Object%20Reference) (OtherActor :type Actor%20Object%20Reference) (OtherComp :type Primitive%20Component%20Object%20Reference) (OtherBodyIndex :type Integer) (bFromSweep :type Boolean) (SweepResult :type Hit%20Result%20Structure%20%28by%20ref%29))
  (bind _asbp_first_person_character (Utilities|Casting|CastToBP_FirstPersonCharacter OtherActor))
  (Variables|Default|SetPlayerRef _asbp_first_person_character)
  (Utilities|FlowControl|DoOnce false
    (:Completed
      (switch Utilities|FlowControl|Switch|SwitchonE_AmmoType (Variables|Default|GetAmmoType)
        (:NewEnumerator0
          (Variables|/Game/FirstPerson/Blueprints/BP_FirstPersonCharacter.BP_FirstPersonCharacter_C|SetBullet (Variables|Default|GetPlayerRef) (Math|Integer|Clamp(Integer) (+ (Variables|/Game/FirstPerson/Blueprints/BP_FirstPersonCharacter.BP_FirstPersonCharacter_C|GetBullet (Variables|Default|GetPlayerRef)) (Variables|Default|GetAmmoToGive)) 0 (Variables|/Game/FirstPerson/Blueprints/BP_FirstPersonCharacter.BP_FirstPersonCharacter_C|GetMaxBullet (Variables|Default|GetPlayerRef))))
          (Default|UpdateBulletAmmo (Variables|/Game/FirstPerson/Blueprints/BP_FirstPersonCharacter.BP_FirstPersonCharacter_C|GetPlayerHUD (Variables|Default|GetPlayerRef)))
          (Audio|PlaySoundatLocation "/Game/SFX/Items/Bullet_Pickup_SFX.Bullet_Pickup_SFX" (Transformation|GetActorLocation) "0, 0, 0" 1.0 1.0 0.0 0 0 0 0)
          (Actor|DestroyActor))
        (:NewEnumerator1
          (Variables|/Game/FirstPerson/Blueprints/BP_FirstPersonCharacter.BP_FirstPersonCharacter_C|SetShell (Variables|Default|GetPlayerRef) (Math|Integer|Clamp(Integer) (+ (Variables|/Game/FirstPerson/Blueprints/BP_FirstPersonCharacter.BP_FirstPersonCharacter_C|GetShell (Variables|Default|GetPlayerRef)) (Variables|Default|GetAmmoToGive)) 0 (Variables|/Game/FirstPerson/Blueprints/BP_FirstPersonCharacter.BP_FirstPersonCharacter_C|GetMaxShell (Variables|Default|GetPlayerRef))))
          (Default|UpdateShellAmmo (Variables|/Game/FirstPerson/Blueprints/BP_FirstPersonCharacter.BP_FirstPersonCharacter_C|GetPlayerHUD (Variables|Default|GetPlayerRef)))
          (Audio|PlaySoundatLocation "/Game/SFX/Items/ShotgunShellsPickup.ShotgunShellsPickup" (Transformation|GetActorLocation) "0, 0, 0" 1.0 1.0 0.0 0 0 0 0)
          (Actor|DestroyActor))
        (:NewEnumerator2
          (Variables|/Game/FirstPerson/Blueprints/BP_FirstPersonCharacter.BP_FirstPersonCharacter_C|SetRocket (Variables|Default|GetPlayerRef) (Math|Integer|Clamp(Integer) (+ (Variables|/Game/FirstPerson/Blueprints/BP_FirstPersonCharacter.BP_FirstPersonCharacter_C|GetRocket (Variables|Default|GetPlayerRef)) (Variables|Default|GetAmmoToGive)) 0 (Variables|/Game/FirstPerson/Blueprints/BP_FirstPersonCharacter.BP_FirstPersonCharacter_C|GetMaxRocket (Variables|Default|GetPlayerRef))))
          (Default|UpdateRocketAmmo (Variables|/Game/FirstPerson/Blueprints/BP_FirstPersonCharacter.BP_FirstPersonCharacter_C|GetPlayerHUD (Variables|Default|GetPlayerRef)))
          (Audio|PlaySoundatLocation "/Game/SFX/Items/RocketPickUp.RocketPickUp" (Transformation|GetActorLocation) "0, 0, 0" 1.0 1.0 0.0 0 0 0 0)
          (Actor|DestroyActor))
        (:NewEnumerator3
          (Variables|/Game/FirstPerson/Blueprints/BP_FirstPersonCharacter.BP_FirstPersonCharacter_C|SetCell (Variables|Default|GetPlayerRef) (Math|Integer|Clamp(Integer) (+ (Variables|/Game/FirstPerson/Blueprints/BP_FirstPersonCharacter.BP_FirstPersonCharacter_C|GetCell (Variables|Default|GetPlayerRef)) (Variables|Default|GetAmmoToGive)) 0 (Variables|/Game/FirstPerson/Blueprints/BP_FirstPersonCharacter.BP_FirstPersonCharacter_C|GetMaxCell (Variables|Default|GetPlayerRef))))
          (Default|UpdateCellAmmo (Variables|/Game/FirstPerson/Blueprints/BP_FirstPersonCharacter.BP_FirstPersonCharacter_C|GetPlayerHUD (Variables|Default|GetPlayerRef)))
          (Actor|DestroyActor)
          (Audio|PlaySoundatLocation "/Game/SFX/Items/CellAmmoPickUp.CellAmmoPickUp" (Transformation|GetActorLocation) "0, 0, 0" 1.0 1.0 0.0 0 0 0 0))))))

(event EventBeginPlay)

(event Collision|EventActorBeginOverlap
  (params (OtherActor :type Actor%20Object%20Reference)))

(event EventTick
  (params (DeltaSeconds :type Float%20%28single-precision%29))
  (Transformation|SetActorRotation (Math|Rotator|MakeRotator 0.0 0.0 (.yaw (Math|Rotator|FindLookatRotation (Transformation|GetActorLocation) (Transformation|GetActorLocation (Game|GetPlayerCharacter 0)))))))

(fn ConstructionScript
  (switch Utilities|FlowControl|Switch|SwitchonE_AmmoType (Variables|Default|GetAmmoType)
    (:NewEnumerator0
      (Rendering|Components|Sprite|SetSprite (Variables|Default|GetPaperSprite) "/Game/Sprites/Item/Bullets_Sprite.Bullets_Sprite"))
    (:NewEnumerator1
      (Rendering|Components|Sprite|SetSprite (Variables|Default|GetPaperSprite) "/Game/Sprites/Item/ShotgunShells_Sprite.ShotgunShells_Sprite"))
    (:NewEnumerator2
      (Rendering|Components|Sprite|SetSprite (Variables|Default|GetPaperSprite) "/Game/Sprites/Item/Rockets_Item_Sprite.Rockets_Item_Sprite"))
    (:NewEnumerator3
      (Rendering|Components|Sprite|SetSprite (Variables|Default|GetPaperSprite) "/Game/Sprites/Item/Cells_Item_Sprite.Cells_Item_Sprite")))
  (Transformation|SetWorldScale3D (Variables|Default|GetPaperSprite) (Variables|Default|GetSpriteSize)))