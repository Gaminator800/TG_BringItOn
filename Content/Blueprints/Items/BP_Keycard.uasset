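; BP_Keycard is a sprite-based keycard pickup that comes in red, orange or blue, set by its Keycard variable.
; The construction script picks the matching Paper2D sprite, and Tick yaws the actor toward the player like a billboard.
; When BP_FirstPersonCharacter overlaps the box, it plays a sound, sets that color's keycard flag on the player, updates the HUD and destroys itself.
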(event OnComponentBeginOverlap(Box)
  (params (OverlappedComponent :type Primitive%20Component%20Object%20Reference) (OtherActor :type Actor%20Object%20Reference) (OtherComp :type Primitive%20Component%20Object%20Reference) (OtherBodyIndex :type Integer) (bFromSweep :type Boolean) (SweepResult :type Hit%20Result%20Structure%20%28by%20ref%29))
  (bind _asbp_first_person_character (Utilities|Casting|CastToBP_FirstPersonCharacter OtherActor))
  (Variables|Default|SetPlayerRef _asbp_first_person_character)
  (Audio|PlaySoundatLocation "/Game/SFX/Items/CardPickUp_SFX.CardPickUp_SFX" (Transformation|GetActorLocation) "0, 0, 0" 1.0 1.0 0.0 0 0 0 0)
  (switch Utilities|FlowControl|Switch|SwitchonE_KeyCard (Variables|Default|GetKeycard)
    (:NewEnumerator0
      (Variables|/Game/FirstPerson/Blueprints/BP_FirstPersonCharacter.BP_FirstPersonCharacter_C|SetRedKeycard? (Variables|Default|GetPlayerRef) true)
      (Default|FindRedkeyCard (Variables|/Game/FirstPerson/Blueprints/BP_FirstPersonCharacter.BP_FirstPersonCharacter_C|GetPlayerHUD (Variables|Default|GetPlayerRef))))
    (:NewEnumerator1
      (Variables|/Game/FirstPerson/Blueprints/BP_FirstPersonCharacter.BP_FirstPersonCharacter_C|SetOrangeKeycard? (Variables|Default|GetPlayerRef) true)
      (Default|FindOrangeKeyCard (Variables|/Game/FirstPerson/Blueprints/BP_FirstPersonCharacter.BP_FirstPersonCharacter_C|GetPlayerHUD (Variables|Default|GetPlayerRef))))
    (:NewEnumerator2
      (Variables|/Game/FirstPerson/Blueprints/BP_FirstPersonCharacter.BP_FirstPersonCharacter_C|SetBlueKeycard? (Variables|Default|GetPlayerRef) true)
      (Default|FindBlueKeyCard (Variables|/Game/FirstPerson/Blueprints/BP_FirstPersonCharacter.BP_FirstPersonCharacter_C|GetPlayerHUD (Variables|Default|GetPlayerRef)))))
  (Actor|DestroyActor))

(event EventBeginPlay)

(event Collision|EventActorBeginOverlap
  (params (OtherActor :type Actor%20Object%20Reference)))

(event EventTick
  (params (DeltaSeconds :type Float%20%28single-precision%29))
  (Transformation|SetActorRotation (Math|Rotator|MakeRotator 0.0 0.0 (.yaw (Math|Rotator|FindLookatRotation (Transformation|GetActorLocation) (Transformation|GetActorLocation (Game|GetPlayerCharacter 0)))))))

(fn ConstructionScript
  (switch Utilities|FlowControl|Switch|SwitchonE_KeyCard (Variables|Default|GetKeycard)
    (:NewEnumerator0
      (Rendering|Components|Sprite|SetSprite (Variables|Default|GetPaperSprite) "/Game/Sprites/Item/RedCardKey_Sprite.RedCardKey_Sprite"))
    (:NewEnumerator1
      (Rendering|Components|Sprite|SetSprite (Variables|Default|GetPaperSprite) "/Game/Sprites/Item/OrangeCardKey_Sprite.OrangeCardKey_Sprite"))
    (:NewEnumerator2
      (Rendering|Components|Sprite|SetSprite (Variables|Default|GetPaperSprite) "/Game/Sprites/Item/BlueCardKey_Sprite.BlueCardKey_Sprite"))))