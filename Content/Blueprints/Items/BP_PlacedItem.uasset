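; BP_PlacedItem is a placeable 2D item actor that turns to face the player like a billboard.
; The construction script applies sprite, flipbook, their world scales and the box extent from variables, so each instance previews in the editor.
; Every tick it sets its rotation to the look-at yaw toward player character 0, leaving pitch and roll at zero.
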(event EventBeginPlay)

(event Collision|EventActorBeginOverlap
  (params (OtherActor :type Actor%20Object%20Reference)))

(event EventTick
  (params (DeltaSeconds :type Float%20%28single-precision%29))
  (Transformation|SetActorRotation (Math|Rotator|MakeRotator 0.0 0.0 (.yaw (Math|Rotator|FindLookatRotation (Transformation|GetActorLocation) (Transformation|GetActorLocation (Game|GetPlayerCharacter 0)))))))

(fn ConstructionScript
  (Utilities|FlowControl|Sequence
    (:then_0
      (Rendering|Components|Sprite|SetSprite (Variables|Default|GetPaperSprite) (Variables|Default|GetSprite))
      (Transformation|SetWorldScale3D (Variables|Default|GetPaperSprite) (Variables|Default|GetSpriteSize)))
    (:then_1
      (Sprite|SetFlipbook (Variables|Default|GetPaperFlipbook) (Variables|Default|GetFlipBook))
      (Transformation|SetWorldScale3D (Variables|Default|GetPaperFlipbook) (Variables|Default|GetFlipBookSize)))
    (:then_2
      (Components|Box|SetBoxExtent (Variables|Default|GetBox) (Variables|Default|GetIn%20Box%20Extent) true))))