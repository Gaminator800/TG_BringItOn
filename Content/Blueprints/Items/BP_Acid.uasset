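; BP_Acid is an acid pool hazard that damages the first-person character over time while they stand in it.
; Entering the Box trigger stores the character and starts a looping timer that calls AcidDamage to apply damage at a fixed interval.
; Leaving the trigger clears that timer through its saved handle.
; The construction script sizes the Acid component and the trigger box from separate variables, PoolSize and InBoxExtent.
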(event OnComponentBeginOverlap(Box)
  (params (OverlappedComponent :type Primitive%20Component%20Object%20Reference) (OtherActor :type Actor%20Object%20Reference) (OtherComp :type Primitive%20Component%20Object%20Reference) (OtherBodyIndex :type Integer) (bFromSweep :type Boolean) (SweepResult :type Hit%20Result%20Structure%20%28by%20ref%29))
  (bind _asbp_first_person_character (Utilities|Casting|CastToBP_FirstPersonCharacter OtherActor))
  (bind _returnvalue (Utilities|Time|SetTimerbyEvent (delegate Custom|AcidDamage) 0.5 true))
  (Variables|Default|SetAcidEvent _returnvalue))

(event OnComponentEndOverlap(Box)
  (params (OverlappedComponent :type Primitive%20Component%20Object%20Reference) (OtherActor :type Actor%20Object%20Reference) (OtherComp :type Primitive%20Component%20Object%20Reference) (OtherBodyIndex :type Integer))
  (Utilities|Casting|CastToBP_FirstPersonCharacter OtherActor)
  (Utilities|Time|ClearandInvalidateTimerbyHandle (Variables|Default|GetAcidEvent)))

(event Custom|AcidDamage
  (Game|Damage|ApplyDamage (stale OnComponentBeginOverlap(Box) _asbp_first_person_character) 1.0 0 0))

(event EventBeginPlay)

(event Collision|EventActorBeginOverlap
  (params (OtherActor :type Actor%20Object%20Reference)))

(event EventTick
  (params (DeltaSeconds :type Float%20%28single-precision%29)))

(fn ConstructionScript
  (Transformation|SetWorldScale3D (Variables|Default|GetAcid) (Variables|Default|GetPoolSize))
  (Components|Box|SetBoxExtent (Variables|Default|GetBox) (Variables|Default|GetIn%20Box%20Extent) true))