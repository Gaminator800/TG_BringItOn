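; BP_KeycardDoor is a color-coded door that opens when the first-person character carries the matching red, orange or blue keycard.
; The construction script sets the cube's material from the KeycardDoor type.
; Box overlap always plays the accepted sound, then checks that card's flag, playing a denied sound on failure.
; On success, a DoOnce-gated timeline raises the cube incrementally from its current height, then destroys the actor.
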(event OnComponentBeginOverlap(Box)
  (params (OverlappedComponent :type Primitive%20Component%20Object%20Reference) (OtherActor :type Actor%20Object%20Reference) (OtherComp :type Primitive%20Component%20Object%20Reference) (OtherBodyIndex :type Integer) (bFromSweep :type Boolean) (SweepResult :type Hit%20Result%20Structure%20%28by%20ref%29))
  (bind _cube (Variables|Default|GetCube))
  (bind _returnvalue (Transformation|GetWorldLocation _cube))
  (bind _asbp_first_person_character (Utilities|Casting|CastToBP_FirstPersonCharacter OtherActor))
  (Variables|Default|SetPlayerRef _asbp_first_person_character)
  (Audio|PlaySoundatLocation "/Game/SFX/Card_Door_Acepted.Card_Door_Acepted" (Transformation|GetActorLocation) "0, 0, 0" 1.0 1.0 0.0 0 0 0 0)
  (switch Utilities|FlowControl|Switch|SwitchonE_KeyCard (Variables|Default|GetKeycardDoor)
    (:NewEnumerator0
      (if (Variables|/Game/FirstPerson/Blueprints/BP_FirstPersonCharacter.BP_FirstPersonCharacter_C|GetRedKeycard? (Variables|Default|GetPlayerRef))
        (Utilities|FlowControl|DoOnce false :!label _label
          (:Completed
            (Audio|PlaySoundatLocation "/Game/SFX/Door_Open_SFX.Door_Open_SFX" (Transformation|GetActorLocation) "0, 0, 0" 1.0 1.0 0.0 0 0 0 0)
            (bind _alpha (Timeline|DoorTL PlayFromStart)
              (:Update
                (Transformation|SetWorldLocation _cube (Math|Vector|MakeVector (.x _returnvalue) (.y _returnvalue) (Math|Float|Lerp (.z _returnvalue) (+ (.z _returnvalue) 15.0) _alpha)) false false))
              (:Finished
                (Utilities|FlowControl|Delay 0.2)
                (Actor|DestroyActor)))))
        (else
          (Audio|PlaySoundatLocation "/Game/SFX/Door_Access_Denied_SFX.Door_Access_Denied_SFX" (Transformation|GetActorLocation) "0, 0, 0" 1.0 1.0 0.0 0 "/Game/SFX/C_DoorKeyCard.C_DoorKeyCard" 0 0 :!label _label_2))))
    (:NewEnumerator1
      (if (Variables|/Game/FirstPerson/Blueprints/BP_FirstPersonCharacter.BP_FirstPersonCharacter_C|GetOrangeKeycard? (Variables|Default|GetPlayerRef))
        (goto _label)
        (else
          (goto _label_2))))
    (:NewEnumerator2
      (if (Variables|/Game/FirstPerson/Blueprints/BP_FirstPersonCharacter.BP_FirstPersonCharacter_C|GetBlueKeycard? (Variables|Default|GetPlayerRef))
        (goto _label)
        (else
          (goto _label_2))))))

(event EventBeginPlay)

(event Collision|EventActorBeginOverlap
  (params (OtherActor :type Actor%20Object%20Reference)))

(event EventTick
  (params (DeltaSeconds :type Float%20%28single-precision%29)))

(fn ConstructionScript
  (switch Utilities|FlowControl|Switch|SwitchonE_KeyCard (Variables|Default|GetKeycardDoor)
    (:NewEnumerator0
      (Rendering|Material|SetMaterial (Variables|Default|GetCube) 0 "/Game/Textures/RedDoor_Mat.RedDoor_Mat"))
    (:NewEnumerator1
      (Rendering|Material|SetMaterial (Variables|Default|GetCube) 0 "/Game/Textures/OrangeDoor_Mat.OrangeDoor_Mat"))
    (:NewEnumerator2
      (Rendering|Material|SetMaterial (Variables|Default|GetCube) 0 "/Game/Textures/BlueDoor_Mat.BlueDoor_Mat"))))