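; Tutorial level-completion trigger that ends the level when the first-person character overlaps its box.
; The one-shot overlap switches the button sprite through a dynamic material parameter and plays the accept sound and completion voice.
; It then disables player input and movement, shows the tutorial win widget with its Level value in UI-only mode with cursor, and stops the game mode timer.
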(event OnComponentBeginOverlap(Box)
  (params (OverlappedComponent :type Primitive%20Component%20Object%20Reference) (OtherActor :type Actor%20Object%20Reference) (OtherComp :type Primitive%20Component%20Object%20Reference) (OtherBodyIndex :type Integer) (bFromSweep :type Boolean) (SweepResult :type Hit%20Result%20Structure%20%28by%20ref%29))
  (bind _returnvalue (Game|GetPlayerController 0))
  (bind _asbp_first_person_character (Utilities|Casting|CastToBP_FirstPersonCharacter OtherActor))
  (Utilities|FlowControl|DoOnce false
    (:Completed
      (bind _returnvalue_2 (Rendering|Material|CreateDynamicMaterialInstance (Variables|Default|GetPlane) 0 "/Game/Textures/ButtonSprite_Mat.ButtonSprite_Mat" "None" :!class /Script/Engine.PrimitiveComponent))
      (Audio|PlaySound2D "/Game/SFX/Card_Door_Acepted.Card_Door_Acepted" 1.0 1.0 0.0 0 0)
      (Audio|PlaySound2D "/Game/SFX/TutorialCompletedVoice.TutorialCompletedVoice" 1.0 1.0 0.0 0 0)
      (Rendering|Material|SetScalarParameterValue _returnvalue_2 "ButtonStateSprite" 1.0 :!class /Script/Engine.MaterialInstanceDynamic)
      (Input|DisableInput _returnvalue)
      (Pawn|Components|CharacterMovement|DisableMovement (Variables|/Script/Engine.Character|GetCharacterMovement _asbp_first_person_character))
      (bind _returnvalue_3 (UserInterface|CreateWidget "/Game/Blueprints/UI/WinScreenTutorial.WinScreenTutorial_C" 0 (Variables|Default|GetLevel)))
      (bind _output_get (Variables|Default|SetWinTutRef _returnvalue_3))
      (Variables|/Script/Engine.PlayerController|SetbShowMouseCursor _returnvalue true)
      (UserInterface|Viewport|AddtoViewport _output_get 0)
      (Input|SetInputModeUIOnly _returnvalue _output_get "DoNotLock" false)
      (Default|TimerStop (Variables|Default|GetGameModeRef)))))

(event EventBeginPlay
  (bind _asbp_first_person_game_mode (Utilities|Casting|CastToBP_FirstPersonGameMode (Game|GetGameMode)))
  (Variables|Default|SetGameModeRef _asbp_first_person_game_mode))

(event Collision|EventActorBeginOverlap
  (params (OtherActor :type Actor%20Object%20Reference)))

(event EventTick
  (params (DeltaSeconds :type Float%20%28single-precision%29)))

(fn ConstructionScript)